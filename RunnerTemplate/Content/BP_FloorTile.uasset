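; Floor tile actor for an endless runner: when the player overlaps its end trigger, it asks the game mode to add another tile, then destroys itself after a short delay.
; The construction script gathers three spawn point transforms and adds a child actor blocker at one chosen at random.
; GetAttachTransform exposes the attach point's world transform.
; SpawnCoins can scatter child actors randomly within the coin area box, but nothing here calls it.
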(event OnComponentBeginOverlap(EndTrigger)
  (params (OverlappedComponent :type Primitive%20Component%20Object%20Reference) (OtherActor :type Actor%20Object%20Reference) (OtherComp :type Primitive%20Component%20Object%20Reference) (OtherBodyIndex :type Integer) (bFromSweep :type Boolean) (SweepResult :type Hit%20Result%20Structure%20%28by%20ref%29))
  (Utilities|Casting|CastToRunplayer OtherActor)
  (bind _asgamemode (Utilities|Casting|CastTogamemode (Game|GetGameMode)))
  (Default|AddFloorTile _asgamemode)
  (Utilities|FlowControl|Delay 2.0)
  (Actor|DestroyActor))

(event EventBeginPlay)

(event Collision|EventActorBeginOverlap
  (params (OtherActor :type Actor%20Object%20Reference)))

(event EventTick
  (params (DeltaSeconds :type Float%20%28single-precision%29)))

(fn ConstructionScript
  (CallFunction|SetSpawnPoints)
  (CallFunction|SpawnBlocker))

(fn GetAttachTransform
  (return (Transformation|GetWorldTransform (Variables|Default|GetAttachPoint))))

(fn SetSpawnPoints
  (Variables|Default|SetSpawn_Point (Utilities|Array|MakeArray (Transformation|GetRelativeTransform (Variables|Default|GetSpawnPoint)) (Transformation|GetRelativeTransform (Variables|Default|GetSpawnPointL)) (Transformation|GetRelativeTransform (Variables|Default|GetSpawnPointR)))))

(fn SpawnBlocker
  (bind _spawn_point (Variables|Default|GetSpawn_Point))
  (AddComponent|AddChildActorComponent false (Utilities|Array|Get(acopy) _spawn_point (Math|Random|RandomIntegerinRange 0 (Utilities|Array|LastIndex _spawn_point)))))

(fn SpawnCoins
  (bind _coinarea (Variables|Default|GetCoinArea))
  (for _index (range 0 5)
    (AddComponent|AddChildActorComponent false (Math|Conversions|ToTransform(Vector) (Math|Random|RandomPointinBoundingBox (Variables|/Script/Engine.SceneComponent|GetRelativeLocation _coinarea) (Variables|/Script/Engine.BoxComponent|GetBoxExtent _coinarea))))))