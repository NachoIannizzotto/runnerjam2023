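; BP_Building3 is a building actor with a Building static mesh and an AttachPoint component.
; GetAttachTransform returns the AttachPoint's world transform.
; An unconnected graph branch would pick one of four Edificio meshes at random, but it never runs, as BeginPlay and the construction script are empty.
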(event EventBeginPlay)

(fn ConstructionScript)

(fn GetAttachTransform
  (return (Transformation|GetWorldTransform (Variables|Default|GetAttachPoint))))